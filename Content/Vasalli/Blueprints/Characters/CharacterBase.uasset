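; CharacterBase is a base character that takes damage with knockback and reports its death to a shared CharacterManager.
; On BeginPlay it finds the existing manager or spawns one, warning if several exist.
; The health interface's Damage event lowers Health, launches the character away from the dealer and shows an animated floating damage widget.
; At zero health or below it notifies the manager with itself and its controller, removes its damage widgets and destroys itself.
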(event EventBeginPlay
  (bind _outactors (Actor|GetAllActorsOfClass "/Game/Vasalli/Blueprints/Characters/CharacterManager.CharacterManager_C"))
  (if (<= (Utilities|Array|Length _outactors) 0)
    (bind _returnvalue (Game|SpawnActorfromClass "/Game/Vasalli/Blueprints/Characters/CharacterManager.CharacterManager_C" (Math|Transform|MakeTransform "0, 0, 0") "Undefined" 0 0))
    (Variables|Default|SetCharacter_Manager_Var _returnvalue)
    (Development|PrintString "MANAGER SPAWNED" true true "(R=1.000000,G=0.000000,B=0.858180,A=1.000000)")
    (else
      (if (> (Utilities|Array|Length _outactors) 1)
        (Development|PrintString "TOO MANY MANAGERS" true true "(R=1.000000,G=0.035793,B=0.000000,A=1.000000)"))
      (Variables|Default|SetCharacter_Manager_Var (Utilities|Array|Get(acopy) _outactors)))))

(event EventHealthInterfaceDamage
  (params (Damage :type Float%20%28single-precision%29) (Dealer :type Actor%20Object%20Reference) (Knock_Back_Degree :type Float%20%28single-precision%29))
  (bind _damage_widgets (Variables|Default|Getdamage_widgets))
  (bind _output_get (Variables|Default|SetHealth (- (Variables|Default|GetHealth) Damage)))
  (Character|LaunchCharacter (* (Math|Vector|Normalize (- (Transformation|GetActorLocation) (Transformation|GetActorLocation Dealer))) Knock_Back_Degree) false false)
  (bind _returnvalue (UserInterface|CreateWidget "/Game/Vasalli/Blueprints/Game/Widget_Text_Damage.Widget_Text_Damage_C" 0 self))
  (Utilities|Array|Add _damage_widgets _returnvalue)
  (UserInterface|Viewport|AddtoViewport _returnvalue 0)
  (UserInterface|Animation|PlayAnimation _returnvalue (Variables|/Game/Vasalli/Blueprints/Game/Widget_Text_Damage.Widget_Text_Damage_C|GetFloating_Text_Ani _returnvalue) 0.0 1 "Forward" 1.0)
  (Variables|/Game/Vasalli/Blueprints/Game/Widget_Text_Damage.Widget_Text_Damage_C|SetFloat%20Damage _returnvalue (* Damage -1.0))
  (if (<= _output_get 0.0)
    (Default|CharacterDied (Variables|Default|GetCharacter_Manager_Var) self (Pawn|GetController))
    (for _array_element _damage_widgets
      (Widget|RemovefromParent _array_element))
    (Actor|DestroyActor)))

(fn ConstructionScript)