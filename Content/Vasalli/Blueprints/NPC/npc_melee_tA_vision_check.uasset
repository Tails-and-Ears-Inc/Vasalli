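; Behavior Tree service that checks whether a melee NPC can see the player and updates its vision state on the Blackboard.
; Each tick, a wide forward-angle test or a close-range fallback gates a camera-channel line trace to the player.
; A sighting sets TargetActor and moves or spawns a TargetPoint marking the last known position.
; Failed checks select a state based on whether that marker exists, which debug mode draws as a sphere.
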(event EventReceiveTickAI
  (params (OwnerController :type AI%20Controller%20Object%20Reference) (ControlledPawn :type Pawn%20Object%20Reference) (DeltaSeconds :type Float%20%28single-precision%29))
  (bind _returnvalue (Transformation|GetActorLocation ControlledPawn))
  (bind _returnvalue_2 (Game|GetPlayerCharacter 0))
  (bind _returnvalue_3 (Game|GetPlayerCharacter 0))
  (bind _last_known_enemy_pos (Variables|Default|Getlast_known_enemy_pos))
  (bind _last_known_enemy_pos_2 (Variables|Default|Getlast_known_enemy_pos))
  (bind _returnvalue_4 (Transformation|GetActorLocation _returnvalue_3))
  (bind _returnvalue_5 (AI|BehaviorTree|GetBlackboardValueasActor _last_known_enemy_pos))
  (bind _returnvalue_6 (AI|BehaviorTree|GetBlackboardValueasActor _last_known_enemy_pos_2))
  (Utilities|FlowControl|Sequence
    (:then_0
      (if (< (Class|KismetMathLibrary|DegAcos (Math|Vector|DotProduct (Math|Vector|Normalize (- _returnvalue_4 _returnvalue)) (Transformation|GetActorForwardVector ControlledPawn))) 158.0)
        (bind _ascharacter (Utilities|Casting|CastToCharacter ControlledPawn :!label _label))
        (bind _outhit (Collision|LineTraceByChannel _returnvalue _returnvalue_4 "TraceTypeQuery2" false (Utilities|Array|MakeArray (Components|GetOwner (Variables|/Script/Engine.Character|GetCapsuleComponent _ascharacter))) "ForDuration"))
        (bind _ascharacter_2 (Utilities|Casting|CastToCharacter (.HitActor (Collision|BreakHitResult _outhit)))
          (:then
            (if (== _ascharacter_2 (Game|GetPlayerCharacter 0))
              (Class|BTFunctionLibrary|SetBlackboardValueasObject (Variables|Default|GetTargetActor) _returnvalue_2)
              (if (!= _returnvalue_5 0)
                (Transformation|SetActorLocation _returnvalue_5 (Transformation|GetActorLocation _returnvalue_2) false false)
                (else
                  (bind _returnvalue_7 (Game|SpawnActorfromClass "/Script/Engine.TargetPoint" (Transformation|GetActorTransform _returnvalue_2) "AlwaysSpawn" 0 0))))
              (Class|BTFunctionLibrary|SetBlackboardValueasObject (Variables|Default|Getlast_known_enemy_pos) _returnvalue_7)
              (Class|BTFunctionLibrary|SetBlackboardValueasEnum (Variables|Default|Getvision_check_State) (Utilities|Enum|Literalenumnpc_melee_tA_state "NewEnumerator1"))
              (else
                (if (!= (AI|BehaviorTree|GetBlackboardValueasActor (Variables|Default|Getlast_known_enemy_pos)) 0) :!label _label_2
                  (Class|BTFunctionLibrary|SetBlackboardValueasEnum (Variables|Default|Getvision_check_State) (Utilities|Enum|Literalenumnpc_melee_tA_state "NewEnumerator2"))
                  (else
                    (Class|BTFunctionLibrary|SetBlackboardValueasEnum (Variables|Default|Getvision_check_State) (Utilities|Enum|Literalenumnpc_melee_tA_state "NewEnumerator0")))))))
          (:CastFailed
            (goto _label_2)))
        (elif (<= (Math|Vector|VectorLength (- _returnvalue_4 _returnvalue)) 128.0)
          (goto _label)
          (else
            (goto _label_2)))))
    (:then_1
      (if (Variables|Default|Getdebug)
        (if (!= _returnvalue_6 0)
          (Rendering|Debug|DrawDebugSphere (Transformation|GetActorLocation _returnvalue_6) 16.0 12 "(R=1.000000,G=0.012164,B=0.000000,A=1.000000)" 1.0 1.0))))))

(event EventReceiveActivationAI
  (params (OwnerController :type AI%20Controller%20Object%20Reference) (ControlledPawn :type Pawn%20Object%20Reference))
  (Class|BTFunctionLibrary|SetBlackboardValueasEnum (Variables|Default|Getvision_check_State) (Utilities|Enum|Literalenumnpc_melee_tA_state "NewEnumerator0")))